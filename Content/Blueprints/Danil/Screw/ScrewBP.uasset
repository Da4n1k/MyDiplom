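; ScrewBP is a screw actor that triggers audio and effects feedback when it hits something.
; One second after BeginPlay it binds a handler to its own OnActorHit event.
; On each hit the handler checks the actor's speed against high and medium thresholds, each with its own activation, followed by a shared one.
; Slower hits trigger nothing.
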(event Custom|OnActorHitImpl
  (params (SelfActor :type Actor%20Object%20Reference) (OtherActor :type Actor%20Object%20Reference) (NormalImpulse :type Vector) (Hit :type Hit%20Result%20Structure%20%28by%20ref%29))
  (bind _returnvalue (Transformation|GetVelocity SelfActor))
  (bind _returnvalue_2 (Math|Vector|VectorLength _returnvalue))
  ;[1 1 1] Audio Effects Collision
  (if (> _returnvalue_2 1e+02)
    (Components|Activation|Activate false)
    (Components|Activation|Activate false :!label _label)
    (elif (> _returnvalue_2 1e+01)
      (Components|Activation|Activate false)
      (goto _label))))

(event EventBeginPlay
  ;[1 1 1] Audio Effects Collision
  (Utilities|FlowControl|Delay 1.0)
  (Collision|AssignOnActorHit (EventDispatchers|CreateEvent :!event Custom|OnActorHitImpl)))

(fn ConstructionScript)