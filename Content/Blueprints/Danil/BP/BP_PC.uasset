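; BP_PC is an actor, apparently a PC prop, that holds references to a VR projector and its projection screen.
; On BeginPlay it turns off physics and collision on its static mesh, then caches the first VRProjectionScreen and VRProjector found in the level.
; A delayed chain to advance the screen and change the slide is unconnected, so it never runs.
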(event EventBeginPlay
  (bind _returnvalue (Actor|GetComponentbyClass "/Script/Engine.StaticMeshComponent"))
  (Physics|SetSimulatePhysics _returnvalue false)
  (Collision|SetCollisionEnabled _returnvalue "NoCollision")
  ;[1 1 1] Finding the Projector Screen
  (bind _outactors (Actor|GetAllActorsOfClass "/Game/Blueprints/Danil/VRStereoProjectionScreen/VRProjectionScreen.VRProjectionScreen_C"))
  (Variables|Default|SetProjectorScreen (Utilities|Array|Get(acopy) _outactors))
  ;[1 1 1] Finding the Projector
  (bind _outactors_2 (Actor|GetAllActorsOfClass "/Game/Blueprints/Danil/VRStereoProjectionScreen/VRProjector.VRProjector_C"))
  (Variables|Default|SetProjector (Utilities|Array|Get(acopy) _outactors_2)))

(event Collision|EventActorBeginOverlap
  (params (OtherActor :type Actor%20Object%20Reference)))

(fn ConstructionScript)