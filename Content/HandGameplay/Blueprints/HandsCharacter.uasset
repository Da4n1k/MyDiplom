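; VR hand-tracking character that flips slides on a projection screen with left and right flick swipe gestures.
; BeginPlay adds the input mapping and caches the first screen and projector found.
; Each Tick, a headset-forward trace gates the gestures, highlights the screen once per look, and sends recognized swipes to screen and projector.
; In-progress gestures drive per-hand timelines that ramp emissive material glow as a cue, reversing otherwise.
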(event Custom|NextS
  (Default|NextScreen (Variables|Default|GetProjectorScreen)))

(event EventBeginPlay
  (|CallParentFunction)
  ;[1 1 1] Add InputMapping context
  (Input|AddMappingContext (PlayerController|LocalPlayerSubsystems|GetEnhancedInputLocalPlayerSubsystem (Game|GetPlayerController 0)) "/Game/HandGameplay/Input/InputMappingContext.InputMappingContext" 0 "(bIgnoreAllPressedKeysUntilRelease=True,bForceImmediately=False,bNotifyUserSettings=False)")
  ;[1 1 1] Finding the Projector Screen
  (bind _outactors (Actor|GetAllActorsOfClass "/Game/Blueprints/Danil/VRStereoProjectionScreen/VRProjectionScreen.VRProjectionScreen_C"))
  (Variables|Default|SetProjectorScreen (Utilities|Array|Get(acopy) _outactors))
  ;[1 1 1] Finding the Projector
  (bind _outactors_2 (Actor|GetAllActorsOfClass "/Game/Blueprints/Danil/VRStereoProjectionScreen/VRProjector.VRProjector_C"))
  (Variables|Default|SetProjector (Utilities|Array|Get(acopy) _outactors_2)))

(event Collision|EventActorBeginOverlap
  (params (OtherActor :type Actor%20Object%20Reference)))

(event EventTick
  (params (DeltaSeconds :type Float%20%28single-precision%29))
  (bind _lefthandtracking (Variables|Default|GetLeftHandTracking))
  (bind _projectorscreen (Variables|Default|GetProjectorScreen))
  (bind _righthandtracking (Variables|Default|GetRightHandTracking))
  (bind _projectorscreen_2 (Variables|Default|GetProjectorScreen))
  (bind _returnvalue (Rendering|Material|GetMaterial _righthandtracking 0))
  (bind _returnvalue_2 (Rendering|Material|GetMaterial _lefthandtracking 0))
  (Utilities|FlowControl|Sequence
    (:then_0
      ;[1 1 1] Screen selection using swipe gestures
      (Utilities|IsLookingatProjectorScreen
        (:Yes
          (Utilities|IsValid _projectorscreen
            (:Is%20Valid
              (if (Variables|Default|GetProjectionScreenHighlightPlayed)
                _
                (else
                  (Default|HighlghtScreen _projectorscreen)
                  (Variables|Default|SetProjectionScreenHighlightPlayed true)))
              (bind _returnvalue_3 (Class|HandGestureRecognizer|GetRecognizedHandGesture (Variables|Default|GetRightFlickSwipeGestureRecognizer) "ResetAll"))
              (if _returnvalue_3
                (Default|NextScreen _projectorscreen_2)
                ;[1 1 1] Projector Light Activates On Page Flips
                (Default|ChangeSlide (Variables|Default|GetProjector) :!label _label)
                (else
                  (bind _returnvalue_4 (Class|HandGestureRecognizer|GetRecognizedHandGesture (Variables|Default|GetLeftFlickSwipeGestureRecognizer) "ResetAll"))
                  (if _returnvalue_4
                    (Default|PreviousScreen _projectorscreen_2)
                    (goto _label)))))))
        (:No
          (Variables|Default|SetProjectionScreenHighlightPlayed false))))
    (:then_1
      ;[1 1 1] Slide Swipe Cues
      (Utilities|IsLookingatProjectorScreen
        (:Yes
          (Utilities|FlowControl|Sequence
            (:then_0
              (bind _returnvalue_5 (Class|HandGestureRecognizer|GetGestureRecognitionState (Variables|Default|GetRightFlickSwipeGestureRecognizer)))
              (if (Utilities|Enum|Equal(Enum) _returnvalue_5 "GestureInProgress")
                ;[1 1 1] Hand highlight cue for hand swipe gesture: lights up when gesture is started
                (bind _emissiverampon1 (Timeline|Шкала%20времени Play)
                  (:Update
                    (Utilities|IsValid _returnvalue
                      (:Is%20Valid
                        (bind _returnvalue_6 (Rendering|Material|CreateDynamicMaterialInstance _righthandtracking 0 _returnvalue "None" :!class /Script/Engine.PrimitiveComponent))
                        (bind _output_get (Variables|Поумолчанию|SetRightHand%20Material%20Instance _returnvalue_6))
                        (Rendering|Material|SetScalarParameterValue _output_get "Emissive" _emissiverampon1 :!class /Script/Engine.MaterialInstanceDynamic)))))
                (else
                  (Timeline|Шкала%20времени Reverse))))
            (:then_1
              (bind _returnvalue_7 (Class|HandGestureRecognizer|GetGestureRecognitionState (Variables|Default|GetLeftFlickSwipeGestureRecognizer)))
              (if (Utilities|Enum|Equal(Enum) _returnvalue_7 "GestureInProgress")
                (bind _emissiverampon2 (Timeline|Шкала%20времени_0 Play)
                  (:Update
                    (Utilities|IsValid _returnvalue_2
                      (:Is%20Valid
                        (bind _returnvalue_8 (Rendering|Material|CreateDynamicMaterialInstance _lefthandtracking 0 _returnvalue_2 "None" :!class /Script/Engine.PrimitiveComponent))
                        (bind _output_get_2 (Variables|Default|SetLeftHand%20Material%20Instance _returnvalue_8))
                        (Rendering|Material|SetScalarParameterValue _output_get_2 "Emissive" _emissiverampon2 :!class /Script/Engine.MaterialInstanceDynamic)))))
                (else
                  (Timeline|Шкала%20времени_0 Reverse))))))
        (:No
          (Utilities|FlowControl|Sequence
            (:then_0
              (Timeline|Шкала%20времени Reverse))
            (:then_1
              (Timeline|Шкала%20времени_0 Reverse))))))))

(fn ConstructionScript
  (|CallParentFunction))